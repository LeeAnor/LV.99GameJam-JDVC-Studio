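; BP_enemy_kl is a flipbook-sprite enemy that attacks by spawning BP_HEAD toward the player and takes its starting HP from BP__Monster_HP.
; Tick halts movement while the player's pause flag is set, otherwise picks attack, walk or death flipbooks.
; The 攻击 event stops it and spawns the head after a delay, while 被伤害 subtracts HP and tints the sprite through a timeline.
; Death decrements the monster count, grants gold, XP and conditional lifesteal, then destroys the actor.
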(event Custom|攻击
  (bind _self self)
  (bind _as_bp_player (Variables|Default|GetAs%20Bp%20Player))
  (bind _charactermovement (Variables|Character|GetCharacterMovement))
  (bind _returnvalue (Transformation|GetActorLocation _as_bp_player))
  (bind _returnvalue_2 (Transformation|GetActorLocation _self))
  (bind _returnvalue_3 (- _returnvalue _returnvalue_2))
  (if (Variables|/Game/blueprints/bp_player.bp_player_C|Get暂停 (Variables|Default|GetAs%20Bp%20Player))
    (Components|Movement|StopMovementImmediately _charactermovement)
    (else
      (Pawn|Components|CharacterMovement|SetMovementMode _charactermovement "MOVE_Walking" 0)
      (Components|Movement|StopMovementImmediately (Variables|Character|GetCharacterMovement))
      (Variables|Default|Set是否攻击 true)
      (Utilities|FlowControl|Delay 2.0)
      (if (not (Variables|Default|Get死亡？))
        (Utilities|IsValid _self
          (:Is%20Valid
            (bind _returnvalue_4 (Game|SpawnActorfromClass "/Game/blueprints/BP_HEAD.BP_HEAD_C" (Math|Transform|MakeTransform (+ (* (Math|Vector|Normalize (Math|Vector|MakeVector (.x _returnvalue_3) (.y _returnvalue_3) 0.0)) (Variables|Default|Get位置)) _returnvalue_2) (Math|Rotator|MakeRotator 0.0 0.0 (.yaw (Math|Rotator|FindLookatRotation _returnvalue_2 _returnvalue)))) "Undefined" 0 0))
            (Utilities|IsValid _returnvalue_4
              (:Is%20Valid
                (Variables|Default|Set是否攻击 false)))))))))

(event Custom|被伤害
  (params (伤害 :type Float%20%28double-precision%29))
  (Variables|Default|SetHP (- (Variables|Default|GetHP) 伤害))
  (bind _color (Timeline|hurt PlayFromStart)
    (:Update
      (Sprite|SetSpriteColor (Variables|Default|GetSprite) _color))))

(event EventBeginPlay
  (bind _outactors (Actor|GetAllActorsOfClass "/Game/ChangeLevel/BP__Monster_HP.BP__Monster_HP_C"))
  (Variables|Default|SetHP (Variables|/Game/ChangeLevel/BP__Monster_HP.BP__Monster_HP_C|GetHP_l (Utilities|Array|Get(acopy) _outactors)))
  (bind _asbp_player (Utilities|Casting|CastTobp_player (Game|GetPlayerCharacter 0)))
  (Variables|Default|SetAs%20Bp%20Player _asbp_player))

(event Collision|EventActorBeginOverlap
  (params (OtherActor :type Actor%20Object%20Reference)))

(event EventTick
  (params (DeltaSeconds :type Float%20%28single-precision%29))
  (bind _returnvalue (Game|GetGameInstance))
  (bind _charactermovement (Variables|Character|GetCharacterMovement))
  (bind _as_bp_player (Variables|Default|GetAs%20Bp%20Player))
  (bind _sprite (Variables|Default|GetSprite))
  (bind _as_bp_player_2 (Variables|Default|GetAs%20Bp%20Player))
  (bind _asbp_gameinstance (Utilities|Casting|CastToBP_GAMEINSTANCE _returnvalue))
  (if (Variables|/Game/blueprints/bp_player.bp_player_C|Get暂停 (Variables|Default|GetAs%20Bp%20Player))
    (Components|Movement|StopMovementImmediately _charactermovement)
    (else
      (Pawn|Components|CharacterMovement|SetMovementMode _charactermovement "MOVE_Walking" 0)
      (if (> (Variables|Default|GetHP) 0.0)
        (if (Variables|Default|Get是否攻击)
          (Sprite|SetFlipbook _sprite "/Game/JDVC/png/enemys/Skeleetons/White/attack/ATTACK_1.ATTACK_1")
          (elif (> (.x (Transformation|GetVelocity)) 0.0)
            (Transformation|SetRelativeRotation _sprite (Math|Rotator|MakeRotator 9e+01 0.0 1.8e+02) false false)
            (Sprite|SetFlipbook _sprite "/Game/JDVC/png/enemys/Skeleetons/White/walk/klxz.klxz")
            (else
              (Transformation|SetRelativeRotation _sprite "0.000000,0.000000,-90.000000" false false)
              (Sprite|SetFlipbook _sprite "/Game/JDVC/png/enemys/Skeleetons/White/walk/klxz.klxz"))))
        (else
          (Variables|Default|Set死亡？ true)
          (Sprite|SetFlipbook (Variables|Default|GetSprite) "/Game/JDVC/2231/enemys/Skeleetons/White/die/kldie.kldie")
          (Components|Movement|StopMovementImmediately (Variables|Character|GetCharacterMovement))
          (Utilities|FlowControl|Delay 1.0)
          (Variables|/Game/blueprints/bp_player.bp_player_C|Set当前怪物 _as_bp_player (- (Variables|/Game/blueprints/bp_player.bp_player_C|Get当前怪物 _as_bp_player) 1))
          (Variables|/Game/全局变量/BP_GAMEINSTANCE.BP_GAMEINSTANCE_C|Set金币 _asbp_gameinstance (+ (Variables|/Game/全局变量/BP_GAMEINSTANCE.BP_GAMEINSTANCE_C|Get金币 _asbp_gameinstance) 2e+01))
          (Variables|/Game/blueprints/bp_player.bp_player_C|Set经验值 _as_bp_player (+ (Variables|/Game/blueprints/bp_player.bp_player_C|Get经验值 _as_bp_player) 20))
          (if (< (Variables|/Game/blueprints/bp_player.bp_player_C|Get当前HP _as_bp_player_2) (Variables|/Game/blueprints/bp_player.bp_player_C|Get最大HP _as_bp_player_2))
            (if (Variables|/Game/blueprints/bp_player.bp_player_C|Get最终吸血 _as_bp_player_2)
              (Variables|/Game/blueprints/bp_player.bp_player_C|Set当前HP _as_bp_player_2 (+ (Variables|/Game/blueprints/bp_player.bp_player_C|Get当前HP _as_bp_player_2) 3.0))))
          (Actor|DestroyActor))))))

(fn ConstructionScript)