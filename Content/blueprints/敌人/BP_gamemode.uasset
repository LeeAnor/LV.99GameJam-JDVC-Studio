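; Game mode that spawns enemies and shows a level-clear UI once the spawn cap is reached and the player's live-enemy count is zero.
; Numeric level names 1–3 set spawn interval, cap and random enemy-type range.
; A Delay on Tick paces EQS queries that pick from the best 25% of locations.
; Each valid result increments the player's enemy count and spawns one of three enemy classes by random roll.
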(event Custom|OnQueryFinishedEvent_事件
  (params (QueryInstance :type Env%20Query%20Instance%20Blueprint%20Wrapper%20Object%20Reference) (QueryStatus :type EEnvQueryStatus%20Enum :default "Processing"))
  (bind _as_bp_player (Variables|Default|GetAs%20Bp%20Player))
  (bind _resultlocations (AI|EQS|GetQueryResultsasLocations QueryInstance))
  (if (AI|IsValidAILocation (Utilities|Array|Get(acopy) _resultlocations))
    (Variables|/Game/blueprints/bp_player.bp_player_C|Set当前怪物 _as_bp_player (+ (Variables|/Game/blueprints/bp_player.bp_player_C|Get当前怪物 _as_bp_player) 1))
    (Variables|Default|Set哪个怪物 (Math|Random|RandomIntegerinRange 0 (Variables|Default|Get怪物)))
    (if (< (Variables|Default|Get哪个怪物) 4)
      (Game|SpawnActorfromClass "/Game/blueprints/敌人/史莱姆1/BP_enemy.BP_enemy_C" (Math|Transform|MakeTransform (Utilities|Array|Get(acopy) _resultlocations)) "Undefined" 0 0)
      (elif (and (> (Variables|Default|Get哪个怪物) 3) (< (Variables|Default|Get哪个怪物) 6))
        (Game|SpawnActorfromClass "/Game/blueprints/敌人/骷髅/BP_enemy_kl.BP_enemy_kl_C" (Math|Transform|MakeTransform (Utilities|Array|Get(acopy) _resultlocations)) "Undefined" 0 0)
        (elif (> (Variables|Default|Get哪个怪物) 5)
          (Game|SpawnActorfromClass "/Game/blueprints/敌人/大怪/2221.2221_C" (Math|Transform|MakeTransform (Utilities|Array|Get(acopy) _resultlocations)) "Undefined" 0 0))))))

(event EventBeginPlay
  (Variables|Default|SetAs%20Bp%20Player (.AsBp%20Player (Utilities|Casting|CastTobp_player (Game|GetPlayerCharacter 0))))
  (bind _returnvalue (UserInterface|CreateWidget "/Game/ESC/UI_ECS_2.UI_ECS_2_C"))
  (bind _output_get (Variables|Default|Set过关UI _returnvalue))
  (Widget|SetVisibility _output_get "Hidden")
  (UserInterface|Viewport|AddtoViewport _output_get 0)
  (bind _returnvalue_2 (Game|GetCurrentLevelName true))
  (if (== (Math|Conversions|ToInteger(Byte) _returnvalue_2) 1)
    (Variables|Default|Set刷怪时间 1.0)
    (Variables|Default|Set最大刷新怪物波数 3e+01)
    (Variables|Default|Set怪物 4)
    (elif (== (Math|Conversions|ToInteger(Byte) _returnvalue_2) 2)
      (Variables|Default|Set刷怪时间 0.5)
      (Variables|Default|Set最大刷新怪物波数 5e+01)
      (Variables|Default|Set怪物 6)
      (elif (== (Math|Conversions|ToInteger(Byte) _returnvalue_2) 3)
        (Variables|Default|Set刷怪时间 0.5)
        (Variables|Default|Set最大刷新怪物波数 1e+02)
        (Variables|Default|Set怪物 8)))))

(event EventTick
  (params (DeltaSeconds :type Float%20%28single-precision%29))
  (if (and (== (Variables|Default|Get刷新怪物波数) (Variables|Default|Get最大刷新怪物波数)) (== (Variables|/Game/blueprints/bp_player.bp_player_C|Get当前怪物 (Variables|Default|GetAs%20Bp%20Player)) 0))
    (Widget|SetVisibility (Variables|Default|Get过关UI) "Visible")
    (Variables|/Script/Engine.PlayerController|SetbShowMouseCursor (Game|GetPlayerController 0) true)
    (else
      (Utilities|FlowControl|Delay (Variables|Default|Get刷怪时间))
      (if (< (Variables|Default|Get刷新怪物波数) (Variables|Default|Get最大刷新怪物波数))
        (bind _result (Math|Float|IncrementFloat (Variables|Default|Get刷新怪物波数))
          (:%20%20
            (Variables|Default|Set刷新怪物波数 _result)
            (bind _returnvalue (AI|EQS|RunEQSQuery "/Game/blueprints/敌人/eqs.eqs" self "RandomBest25Pct"))
            (Variables|Default|SetEQS _returnvalue)
            (EventDispatchers|AssignOnQueryFinishedEvent (Variables|Default|GetEQS) (delegate Custom|OnQueryFinishedEvent_事件))))))))

(fn ConstructionScript)