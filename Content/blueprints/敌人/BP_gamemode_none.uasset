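; BP_gamemode_none is, by its name, a game mode without enemy spawning: its events are empty and all spawn logic is disconnected.
; The unused wave logic waits a delay, increments a capped wave counter and runs a random-best-25% EQS query.
; Its disconnected result logic would spawn one of three randomly chosen enemy classes at the first returned location, if valid.
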(event Custom|OnQueryFinishedEvent_事件
  (params (QueryInstance :type Env%20Query%20Instance%20Blueprint%20Wrapper%20Object%20Reference) (QueryStatus :type EEnvQueryStatus%20Enum :default "Processing")))

(event EventTick
  (params (DeltaSeconds :type Float%20%28single-precision%29)))

(fn ConstructionScript)