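; Flipbook-based slime enemy that damages the player and grants rewards when killed.
; On BeginPlay it copies HP from the first BP__Monster_HP actor; the damage event subtracts from it and plays a sprite color timeline.
; Tick polls the player's pause flag and HP, playing death, then awarding gold, XP and conditional lifesteal, decrementing monster count and self-destroying.
; The attack event halts movement, then damages the player after a delay if still alive.
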(event Custom|攻击
  (bind _as_bp_player (Variables|Default|GetAs%20Bp%20Player))
  (if (Variables|/Game/blueprints/bp_player.bp_player_C|Get暂停 (Variables|Default|GetAs%20Bp%20Player))
    (Components|Movement|StopMovementImmediately (Variables|Character|GetCharacterMovement))
    (else
      (Pawn|Components|CharacterMovement|SetMovementMode (Variables|Character|GetCharacterMovement) "MOVE_Walking" 0)
      (Components|Movement|StopMovementImmediately (Variables|Character|GetCharacterMovement))
      (Utilities|FlowControl|Delay 0.5)
      (if (not (Variables|Default|Get在死亡状态吗？))
        (Utilities|IsValid self
          (:Is%20Valid
            (Variables|/Game/blueprints/bp_player.bp_player_C|Set当前HP _as_bp_player (- (Variables|/Game/blueprints/bp_player.bp_player_C|Get当前HP _as_bp_player) (Variables|Default|Get伤害)))))))))

(event Custom|被伤害
  (params (伤害 :type Float%20%28double-precision%29))
  (Variables|Default|SetHP (- (Variables|Default|GetHP) 伤害))
  (bind _color (Timeline|Timeline PlayFromStart)
    (:Update
      (Sprite|SetSpriteColor (Variables|Default|GetSprite) _color))))

(event EventBeginPlay
  (bind _outactors (Actor|GetAllActorsOfClass "/Game/ChangeLevel/BP__Monster_HP.BP__Monster_HP_C"))
  (Variables|Default|SetHP (Variables|/Game/ChangeLevel/BP__Monster_HP.BP__Monster_HP_C|GetHP_l (Utilities|Array|Get(acopy) _outactors)))
  (bind _asbp_player (Utilities|Casting|CastTobp_player (Game|GetPlayerCharacter 0)))
  (Variables|Default|SetAs%20Bp%20Player _asbp_player))

(event Collision|EventActorBeginOverlap
  (params (OtherActor :type Actor%20Object%20Reference)))

(event EventTick
  (params (DeltaSeconds :type Float%20%28single-precision%29))
  (bind _returnvalue (Game|GetGameInstance))
  (bind _as_bp_player (Variables|Default|GetAs%20Bp%20Player))
  (bind _as_bp_player_2 (Variables|Default|GetAs%20Bp%20Player))
  (bind _asbp_gameinstance (Utilities|Casting|CastToBP_GAMEINSTANCE _returnvalue))
  (if (Variables|/Game/blueprints/bp_player.bp_player_C|Get暂停 (Variables|Default|GetAs%20Bp%20Player))
    (Components|Movement|StopMovementImmediately (Variables|Character|GetCharacterMovement))
    (else
      (Pawn|Components|CharacterMovement|SetMovementMode (Variables|Character|GetCharacterMovement) "MOVE_Walking" 0)
      (if (not (> (Variables|Default|GetHP) 0.0))
        (Variables|Default|Set在死亡状态吗？ true)
        (Sprite|SetFlipbook (Variables|Default|GetSprite) "/Game/JDVC/2231/enemys/Slime/GreenSlime/die/slmdie.slmdie")
        (Components|Movement|StopMovementImmediately (Variables|Character|GetCharacterMovement))
        (Utilities|FlowControl|Delay 1.0)
        (Variables|/Game/全局变量/BP_GAMEINSTANCE.BP_GAMEINSTANCE_C|Set金币 _asbp_gameinstance (+ (Variables|/Game/全局变量/BP_GAMEINSTANCE.BP_GAMEINSTANCE_C|Get金币 _asbp_gameinstance) 1e+01))
        (Variables|/Game/blueprints/bp_player.bp_player_C|Set当前怪物 _as_bp_player (- (Variables|/Game/blueprints/bp_player.bp_player_C|Get当前怪物 _as_bp_player) 1))
        (Variables|/Game/blueprints/bp_player.bp_player_C|Set经验值 _as_bp_player (+ (Variables|/Game/blueprints/bp_player.bp_player_C|Get经验值 _as_bp_player) 10))
        (if (< (Variables|/Game/blueprints/bp_player.bp_player_C|Get当前HP _as_bp_player_2) (Variables|/Game/blueprints/bp_player.bp_player_C|Get最大HP _as_bp_player_2))
          (if (Variables|/Game/blueprints/bp_player.bp_player_C|Get最终吸血 _as_bp_player_2)
            (Variables|/Game/blueprints/bp_player.bp_player_C|Set当前HP _as_bp_player_2 (+ (Variables|/Game/blueprints/bp_player.bp_player_C|Get当前HP _as_bp_player_2) 3.0))))
        (Actor|DestroyActor)))))

(fn ConstructionScript)