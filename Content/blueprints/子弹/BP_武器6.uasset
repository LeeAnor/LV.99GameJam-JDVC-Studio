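; BP_武器6 (Weapon 6) is a weapon Blueprint that fires a bullet for the player when its WeaponAttack01 event runs.
; The event spawns BP_子弹 at the player's 变换位置 transform and passes in the player's 武器状态 weapon state.
; A valid bullet is then rotated with a fixed roll and a yaw taken from the player's 偏移浮点 offset.
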(event EventBeginPlay
  (|CallParentFunction) ; 此节点被禁用，将不会被调用。\n从引脚连出引线来编译功能。
)

(event Collision|EventActorBeginOverlap
  (params (OtherActor :type Actor%20Object%20Reference))
  (|CallParentFunction OtherActor) ; 此节点被禁用，将不会被调用。\n从引脚连出引线来编译功能。
)

(event EventTick
  (params (DeltaSeconds :type Float%20%28single-precision%29))
  (|CallParentFunction DeltaSeconds) ; 此节点被禁用，将不会被调用。\n从引脚连出引线来编译功能。
)

(event EventWeaponAttack01
  (bind _returnvalue (Game|GetPlayerCharacter 0))
  (bind _asbp_player (Utilities|Casting|CastTobp_player _returnvalue))
  (Utilities|FlowControl|Sequence
    (:then_0
      (Variables|Default|SetAs%20Bp%20Player _asbp_player)
      (bind _returnvalue_2 (Game|SpawnActorfromClass "/Game/blueprints/BP_子弹.BP_子弹_C" (Variables|/Game/blueprints/bp_player.bp_player_C|Get变换位置 _asbp_player) "Undefined" 0 (Variables|/Game/blueprints/bp_player.bp_player_C|Get武器状态 _asbp_player) 0))
      (Utilities|IsValid _returnvalue_2
        (:Is%20Valid
          (Transformation|SetActorRotation _returnvalue_2 (Math|Rotator|MakeRotator -9e+01 0.0 (Variables|/Game/blueprints/bp_player.bp_player_C|Get偏移浮点 _asbp_player))))))))

(fn ConstructionScript
  (|CallParentFunction))