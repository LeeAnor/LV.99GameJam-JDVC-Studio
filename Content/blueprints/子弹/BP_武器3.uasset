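; BP_武器3 is a weapon Blueprint in the bullet folder, shown through a PaperFlipbook component.
; Every Tick it casts the player character to bp_player and reads 开火子弹可视 (fire bullet visible), hiding the flipbook when true and showing it otherwise.
; The WeaponAttack01 event clears the 攻击 (attack) flag.
; BeginPlay, overlap and construction add no logic of their own.
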(event EventBeginPlay
  (|CallParentFunction) ; 此节点被禁用，将不会被调用。\n从引脚连出引线来编译功能。
)

(event Collision|EventActorBeginOverlap
  (params (OtherActor :type Actor%20Object%20Reference))
  (|CallParentFunction OtherActor) ; 此节点被禁用，将不会被调用。\n从引脚连出引线来编译功能。
)

(event EventWeaponAttack01
  (Variables|Default|Set攻击 false))

(event EventTick
  (params (DeltaSeconds :type Float%20%28single-precision%29))
  (bind _paperflipbook (Variables|Default|GetPaperFlipbook))
  (if (Variables|/Game/blueprints/bp_player.bp_player_C|Get开火子弹可视 (.AsBp%20Player (Utilities|Casting|CastTobp_player (Game|GetPlayerCharacter 0))))
    (Rendering|SetVisibility _paperflipbook false false)
    (else
      (Rendering|SetVisibility _paperflipbook true false))))

(fn ConstructionScript
  (|CallParentFunction))