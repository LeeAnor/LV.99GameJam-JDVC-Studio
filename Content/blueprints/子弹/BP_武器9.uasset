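; BP_武器9 is a weapon Blueprint whose WeaponAttack01 event fires a three-bullet fan from the player.
; It reads spawn position, aim yaw and weapon state from bp_player, passing that state into each BP_子弹.
; Bullets spawn at center, +10 and -10 degrees yaw, each rolled -90 degrees.
; Each follow-up spawn runs only if the previous bullet is valid.
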(event EventBeginPlay
  (|CallParentFunction) ; 此节点被禁用，将不会被调用。\n从引脚连出引线来编译功能。
)

(event Collision|EventActorBeginOverlap
  (params (OtherActor :type Actor%20Object%20Reference))
  (|CallParentFunction OtherActor) ; 此节点被禁用，将不会被调用。\n从引脚连出引线来编译功能。
)

(event EventTick
  (params (DeltaSeconds :type Float%20%28single-precision%29))
  (|CallParentFunction DeltaSeconds) ; 此节点被禁用，将不会被调用。\n从引脚连出引线来编译功能。
)

(event EventWeaponAttack01
  (bind _returnvalue (Game|GetPlayerCharacter 0))
  (bind _asbp_player (Utilities|Casting|CastTobp_player _returnvalue))
  (bind _子弹向量位置 (Variables|/Game/blueprints/bp_player.bp_player_C|Get子弹向量位置 _asbp_player))
  (bind _偏移浮点 (Variables|/Game/blueprints/bp_player.bp_player_C|Get偏移浮点 _asbp_player))
  (bind _武器状态 (Variables|/Game/blueprints/bp_player.bp_player_C|Get武器状态 _asbp_player))
  (bind _returnvalue_2 (+ _偏移浮点 1e+01))
  (bind _returnvalue_3 (- _偏移浮点 1e+01))
  (Utilities|FlowControl|Sequence
    (:then_0
      (Variables|Default|SetAs%20Bp%20Player _asbp_player)
      (bind _returnvalue_4 (Game|SpawnActorfromClass "/Game/blueprints/BP_子弹.BP_子弹_C" (Math|Transform|MakeTransform _子弹向量位置 (Math|Rotator|MakeRotator 0.0 0.0 _偏移浮点)) "Undefined" 0 _武器状态 0))
      (Utilities|IsValid _returnvalue_4
        (:Is%20Valid
          (Transformation|SetActorRotation _returnvalue_4 (Math|Rotator|MakeRotator -9e+01 0.0 _偏移浮点))
          (bind _returnvalue_5 (Game|SpawnActorfromClass "/Game/blueprints/BP_子弹.BP_子弹_C" (Math|Transform|MakeTransform _子弹向量位置 (Math|Rotator|MakeRotator 0.0 0.0 _returnvalue_2)) "Undefined" 0 _武器状态 0))
          (Utilities|IsValid _returnvalue_5
            (:Is%20Valid
              (Transformation|SetActorRotation _returnvalue_5 (Math|Rotator|MakeRotator -9e+01 0.0 _returnvalue_2))
              (bind _returnvalue_6 (Game|SpawnActorfromClass "/Game/blueprints/BP_子弹.BP_子弹_C" (Math|Transform|MakeTransform _子弹向量位置 (Math|Rotator|MakeRotator 0.0 0.0 _returnvalue_3)) "Undefined" 0 _武器状态 0))
              (Utilities|IsValid _returnvalue_6
                (:Is%20Valid
                  (Transformation|SetActorRotation _returnvalue_6 (Math|Rotator|MakeRotator -9e+01 0.0 _returnvalue_3)))))))))))

(fn ConstructionScript
  (|CallParentFunction))