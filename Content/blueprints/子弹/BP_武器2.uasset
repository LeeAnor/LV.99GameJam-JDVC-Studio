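; Second weapon actor that fires BP_子弹 bullets for the player character and shows a flipbook while firing.
; WeaponAttack01 spawns a bullet at the player's 变换位置 transform, passes in the player's 武器状态, and rotates it by -90 roll with yaw from 偏移浮点.
; Tick polls the player's 开火子弹可视 flag each frame to toggle PaperFlipbook1 visibility.
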(event EventBeginPlay
  (|CallParentFunction) ; 此节点被禁用，将不会被调用。\n从引脚连出引线来编译功能。
)

(event Collision|EventActorBeginOverlap
  (params (OtherActor :type Actor%20Object%20Reference))
  (|CallParentFunction OtherActor) ; 此节点被禁用，将不会被调用。\n从引脚连出引线来编译功能。
)

(event EventWeaponAttack01
  (bind _returnvalue (Game|GetPlayerCharacter 0))
  (bind _asbp_player (Utilities|Casting|CastTobp_player _returnvalue))
  (Variables|Default|Set获取玩家角色 _asbp_player)
  (bind _returnvalue_2 (Game|SpawnActorfromClass "/Game/blueprints/BP_子弹.BP_子弹_C" (Variables|/Game/blueprints/bp_player.bp_player_C|Get变换位置 _asbp_player) "Undefined" 0 (Variables|/Game/blueprints/bp_player.bp_player_C|Get武器状态 _asbp_player) 0))
  (Utilities|IsValid _returnvalue_2
    (:Is%20Valid
      (Transformation|SetActorRotation _returnvalue_2 (Math|Rotator|MakeRotator -9e+01 0.0 (Variables|/Game/blueprints/bp_player.bp_player_C|Get偏移浮点 _asbp_player))))))

(event EventTick
  (params (DeltaSeconds :type Float%20%28single-precision%29))
  (bind _paperflipbook1 (Variables|Default|GetPaperFlipbook1))
  (if (Variables|/Game/blueprints/bp_player.bp_player_C|Get开火子弹可视 (.AsBp%20Player (Utilities|Casting|CastTobp_player (Game|GetPlayerCharacter 0))))
    (Rendering|SetVisibility _paperflipbook1 true false)
    (else
      (Rendering|SetVisibility _paperflipbook1 false false))))

(fn ConstructionScript
  (|CallParentFunction))