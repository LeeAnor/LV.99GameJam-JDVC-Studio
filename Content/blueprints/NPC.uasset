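; NPC actor that lets the player start a dialogue by pressing I while inside its trigger box.
; On begin play it writes its name to the 对话 widget component and adds a collapsed 与NPC1对话 dialogue to the viewport.
; Box overlaps toggle the prompt and actor input; I disables movement and look, then shows the dialogue and cursor.
; Tick polls bp_player's 对话结束了 flag to collapse the dialogue.
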(event OnComponentBeginOverlap(Box)
  (params (OverlappedComponent :type Primitive%20Component%20Object%20Reference) (OtherActor :type Actor%20Object%20Reference) (OtherComp :type Primitive%20Component%20Object%20Reference) (OtherBodyIndex :type Integer) (bFromSweep :type Boolean) (SweepResult :type Hit%20Result%20Structure%20%28by%20ref%29))
  (Utilities|Casting|CastTobp_player OtherActor)
  (Utilities|FlowControl|DoOnce false :!label _label
    (:Completed
      (Rendering|SetVisibility (Variables|Default|GetWidget) true false)
      (Variables|Default|Set是否在里面 true)
      (Input|EnableInput (Game|GetPlayerController 0))
      (goto _label Reset))))

(event OnComponentEndOverlap(Box)
  (params (OverlappedComponent :type Primitive%20Component%20Object%20Reference) (OtherActor :type Actor%20Object%20Reference) (OtherComp :type Primitive%20Component%20Object%20Reference) (OtherBodyIndex :type Integer))
  (Utilities|Casting|CastTobp_player OtherActor)
  (Rendering|SetVisibility (Variables|Default|GetWidget) false false)
  (Variables|Default|Set是否在里面 false)
  (Input|DisableInput (Game|GetPlayerController 0)))

(event EventBeginPlay
  (bind _as对话 (Utilities|Casting|CastTo对话 (UserInterface|GetUserWidgetObject (Variables|Default|GetWidget))))
  (Rendering|Components|TextRender|SetText (Variables|/Game/UMG界面/对话系统/对话.对话_C|GetNAME _as对话) (Variables|Default|Getname))
  (bind _returnvalue (UserInterface|CreateWidget "/Game/UMG界面/对话系统/与NPC1对话.与NPC1对话_C"))
  (bind _output_get (Variables|Default|SetNPC1映射 _returnvalue))
  (Widget|SetVisibility _output_get "Collapsed")
  (UserInterface|Viewport|AddtoViewport (Variables|Default|GetNPC1映射) 0))

(event Collision|EventActorBeginOverlap
  (params (OtherActor :type Actor%20Object%20Reference)))

(event EventTick
  (params (DeltaSeconds :type Float%20%28single-precision%29))
  (bind _returnvalue (Game|GetPlayerCharacter 0))
  (bind _asbp_player (Utilities|Casting|CastTobp_player _returnvalue))
  (if (Variables|/Game/blueprints/bp_player.bp_player_C|Get对话结束了 _asbp_player)
    (Variables|/Game/blueprints/bp_player.bp_player_C|Set对话结束了 _asbp_player false)
    (Widget|SetVisibility (Variables|Default|GetNPC1映射) "Collapsed")))

(event Input|KeyboardEvents|I
  (params (Key :type Key%20Structure :default "None"))
  (:Pressed
    (Pawn|Components|CharacterMovement|DisableMovement (Variables|/Script/Engine.Character|GetCharacterMovement (Game|GetPlayerCharacter 0)))
    (Input|SetIgnoreLookInput (Game|GetPlayerController 0) true)
    (Rendering|SetVisibility (Variables|Default|GetWidget) false false)
    (Widget|SetVisibility (Variables|Default|GetNPC1映射) "Visible")
    (Variables|/Script/Engine.PlayerController|SetbShowMouseCursor (.AsBp%20Playercontrol (Utilities|Casting|CastTobp_playercontrol (Game|GetPlayerController 0))) true)))

(fn ConstructionScript)