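; BP_HEAD is a short-lived projectile actor that damages the player on contact.
; The construction script sets the ProjectileMovement initial speed, and a Delay on Tick destroys the actor after about two seconds.
; When its Box overlaps the Box1 component of bp_player, it subtracts 伤害 (damage) from the player's 当前HP (current HP) and destroys itself.
; BeginPlay also stores a player reference, which the overlap logic does not use.
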(event OnComponentBeginOverlap(Box)
  (params (OverlappedComponent :type Primitive%20Component%20Object%20Reference) (OtherActor :type Actor%20Object%20Reference) (OtherComp :type Primitive%20Component%20Object%20Reference) (OtherBodyIndex :type Integer) (bFromSweep :type Boolean) (SweepResult :type Hit%20Result%20Structure%20%28by%20ref%29))
  (bind _asbp_player (Utilities|Casting|CastTobp_player OtherActor))
  (if (== (Variables|/Game/blueprints/bp_player.bp_player_C|GetBox1 _asbp_player) OtherComp)
    (Variables|/Game/blueprints/bp_player.bp_player_C|Set当前HP _asbp_player (- (Variables|/Game/blueprints/bp_player.bp_player_C|Get当前HP _asbp_player) (Variables|Default|Get伤害)))
    (Actor|DestroyActor)))

(event EventBeginPlay
  (Variables|Default|SetAs%20Bp%20Player (.AsBp%20Player (Utilities|Casting|CastTobp_player (Game|GetPlayerCharacter 0)))))

(event EventTick
  (params (DeltaSeconds :type Float%20%28single-precision%29))
  (Utilities|FlowControl|Delay 2.0)
  (Actor|DestroyActor))

(event Collision|EventActorBeginOverlap
  (params (OtherActor :type Actor%20Object%20Reference)))

(fn ConstructionScript
  (Variables|/Script/Engine.ProjectileMovementComponent|SetInitialSpeed (Variables|Default|GetProjectileMovement) 1e+02))