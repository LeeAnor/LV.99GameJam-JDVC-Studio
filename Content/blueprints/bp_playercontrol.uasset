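; Player controller that manages the game's menus: inventory (W_菜单), item bag, shop and ESC menu.
; BeginPlay pre-creates them hidden, plus a second UI_ECS (过关) that is never shown here.
; Debounced inputs toggle one menu at a time via pause flags, with the item key opening the shop inside shops.
; Toggles switch movement, look input and cursor; bp_player.暂停 flips even when another menu blocks the toggle.
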(event Custom|切换背包
  (bind _returnvalue (Game|GetPlayerCharacter 0))
  (bind _库存菜单ref (Variables|Default|Get库存菜单ref))
  (bind _charactermovement (Variables|/Script/Engine.Character|GetCharacterMovement _returnvalue))
  (if (Variables|Default|Get暂停)
    (Variables|Default|Set暂停 false)
    (Pawn|Components|CharacterMovement|SetMovementMode _charactermovement "MOVE_Walking" 0)
    (Input|ResetIgnoreLookInput)
    (Widget|SetVisibility _库存菜单ref "Collapsed")
    (Variables|Default|SetbShowMouseCursor false)
    (Input|SetInputModeGameOnly self true)
    (else
      (Variables|Default|Set暂停 true)
      (Pawn|Components|CharacterMovement|DisableMovement _charactermovement)
      (Input|SetIgnoreLookInput true)
      (Widget|SetVisibility _库存菜单ref "SelfHitTestInvisible")
      (Variables|Default|SetbShowMouseCursor true))))

(event Custom|切换商店
  (bind _returnvalue (Game|GetPlayerCharacter 0))
  (bind _商店菜单 (Variables|Default|Get商店菜单))
  (bind _charactermovement (Variables|/Script/Engine.Character|GetCharacterMovement _returnvalue))
  (if (Variables|Default|Get商店暂停)
    (Variables|Default|Set商店暂停 false)
    (Pawn|Components|CharacterMovement|SetMovementMode _charactermovement "MOVE_Walking" 0)
    (Input|ResetIgnoreLookInput)
    (Widget|SetVisibility _商店菜单 "Collapsed")
    (Input|SetInputModeGameOnly self true)
    (Variables|Default|SetbShowMouseCursor false)
    (else
      (Variables|Default|Set商店暂停 true)
      (Pawn|Components|CharacterMovement|DisableMovement _charactermovement)
      (Input|SetIgnoreLookInput true)
      (Widget|SetVisibility _商店菜单 "SelfHitTestInvisible")
      (Variables|Default|SetbShowMouseCursor true))))

(event Custom|切换物品
  (bind _returnvalue (Game|GetPlayerCharacter 0))
  (bind _背包菜单 (Variables|Default|Get背包菜单))
  (bind _charactermovement (Variables|/Script/Engine.Character|GetCharacterMovement _returnvalue))
  (if (Variables|Default|Get物品暂停)
    (Variables|Default|Set物品暂停 false)
    (Pawn|Components|CharacterMovement|SetMovementMode _charactermovement "MOVE_Walking" 0)
    (Input|ResetIgnoreLookInput)
    (Widget|SetVisibility _背包菜单 "Collapsed")
    (Input|SetInputModeGameOnly self true)
    (Variables|Default|SetbShowMouseCursor false)
    (else
      (Variables|Default|Set物品暂停 true)
      (Pawn|Components|CharacterMovement|DisableMovement _charactermovement)
      (Input|SetIgnoreLookInput true)
      (Widget|SetVisibility _背包菜单 "Visible")
      (Variables|Default|SetbShowMouseCursor true))))

(event Custom|切换菜单
  (bind _returnvalue (Game|GetPlayerCharacter 0))
  (bind _ui (Variables|Default|GetUI))
  (bind _charactermovement (Variables|/Script/Engine.Character|GetCharacterMovement _returnvalue))
  (if (Variables|Default|GetUI暂停)
    (Variables|Default|SetUI暂停 false)
    (Pawn|Components|CharacterMovement|SetMovementMode _charactermovement "MOVE_Walking" 0)
    (Input|ResetIgnoreLookInput)
    (Widget|SetVisibility _ui "Hidden")
    (Input|SetInputModeGameOnly self true)
    (Variables|Default|SetbShowMouseCursor false)
    (else
      (Variables|Default|SetUI暂停 true)
      (Pawn|Components|CharacterMovement|DisableMovement _charactermovement)
      (Input|SetIgnoreLookInput true)
      (Widget|SetVisibility _ui "Visible")
      (Variables|Default|SetbShowMouseCursor true))))

(event Input|EnhancedActionEvents|EnhancedInputAction开启ESC
  (params (ActionValue :type Boolean) (ElapsedSeconds :type Float%20%28double-precision%29) (TriggeredSeconds :type Float%20%28double-precision%29) (InputAction :type Input%20Action%20Object%20Reference :default "/Game/input/开启ESC.开启ESC"))
  (bind _returnvalue (Game|GetPlayerCharacter 0))
  (bind _asbp_player (Utilities|Casting|CastTobp_player _returnvalue))
  (:Triggered
    (Utilities|FlowControl|DoOnce false :!label _label
      (:Completed
        (if (Variables|/Game/blueprints/bp_player.bp_player_C|Get暂停 _asbp_player)
          (Variables|/Game/blueprints/bp_player.bp_player_C|Set暂停 _asbp_player false)
          (else
            (Variables|/Game/blueprints/bp_player.bp_player_C|Set暂停 _asbp_player true)))
        (if (not (or (or (Variables|Default|Get暂停) (Variables|Default|Get物品暂停)) (Variables|Default|Get商店暂停)))
          (CallFunction|切换菜单)))))
  (:Completed
    (goto _label Reset)))

(event Input|EnhancedActionEvents|EnhancedInputAction开启背包
  (params (ActionValue :type Boolean) (ElapsedSeconds :type Float%20%28double-precision%29) (TriggeredSeconds :type Float%20%28double-precision%29) (InputAction :type Input%20Action%20Object%20Reference :default "/Game/input/开启背包.开启背包"))
  (bind _returnvalue (Game|GetPlayerCharacter 0))
  (bind _asbp_player (Utilities|Casting|CastTobp_player _returnvalue))
  ;[1 1 1] 切换背包
  (:Triggered
    (Utilities|FlowControl|DoOnce false :!label _label
      (:Completed
        (if (Variables|/Game/blueprints/bp_player.bp_player_C|Get暂停 _asbp_player)
          (Variables|/Game/blueprints/bp_player.bp_player_C|Set暂停 _asbp_player false)
          (else
            (Variables|/Game/blueprints/bp_player.bp_player_C|Set暂停 _asbp_player true)))
        (if (not (or (Variables|Default|GetUI暂停) (or (Variables|Default|Get物品暂停) (Variables|Default|Get商店暂停))))
          (CallFunction|切换背包)))))
  (:Completed
    (goto _label Reset)))

(event Input|EnhancedActionEvents|EnhancedInputAction开启物品背包
  (params (ActionValue :type Boolean) (ElapsedSeconds :type Float%20%28double-precision%29) (TriggeredSeconds :type Float%20%28double-precision%29) (InputAction :type Input%20Action%20Object%20Reference :default "/Game/input/开启物品背包.开启物品背包"))
  (bind _returnvalue (Game|GetPlayerCharacter 0))
  (bind _returnvalue_2 (Game|GetPlayerCharacter 0))
  (bind _asbp_player (Utilities|Casting|CastTobp_player _returnvalue))
  (bind _asbp_player_2 (Utilities|Casting|CastTobp_player _returnvalue_2))
  (bind _是否在商店中 (Variables|/Game/blueprints/bp_player.bp_player_C|Get是否在商店中 _asbp_player))
  (:Triggered
    (if _是否在商店中
      (Utilities|FlowControl|DoOnce false :!label _label
        (:Completed
          (if (Variables|/Game/blueprints/bp_player.bp_player_C|Get暂停 _asbp_player_2)
            (Variables|/Game/blueprints/bp_player.bp_player_C|Set暂停 _asbp_player_2 false)
            (else
              (Variables|/Game/blueprints/bp_player.bp_player_C|Set暂停 _asbp_player_2 true)))
          (if (not (or (Variables|Default|GetUI暂停) (or (Variables|Default|Get暂停) (Variables|Default|Get物品暂停))))
            (CallFunction|切换商店))))
      (else
        (Utilities|FlowControl|DoOnce false :!label _label_2
          (:Completed
            (if (Variables|/Game/blueprints/bp_player.bp_player_C|Get暂停 _asbp_player_2)
              (Variables|/Game/blueprints/bp_player.bp_player_C|Set暂停 _asbp_player_2 false)
              (else
                (Variables|/Game/blueprints/bp_player.bp_player_C|Set暂停 _asbp_player_2 true)))
            (if (not (or (Variables|Default|GetUI暂停) (or (Variables|Default|Get商店暂停) (Variables|Default|Get暂停))))
              (CallFunction|切换物品)))))))
  (:Completed
    (if _是否在商店中
      (goto _label Reset)
      (else
        (goto _label_2 Reset)))))

(event EventBeginPlay
  (Utilities|FlowControl|Sequence
    (:then_0
      (bind _returnvalue (UserInterface|CreateWidget "/Game/UMG界面/W_菜单.W_菜单_C"))
      (bind _output_get (Variables|Default|Set库存菜单ref _returnvalue))
      (Widget|SetVisibility _output_get "Collapsed")
      (UserInterface|Viewport|AddtoViewport (Variables|Default|Get库存菜单ref) 0))
    (:then_1
      (bind _returnvalue_2 (UserInterface|CreateWidget "/Game/UMG界面/药品界面/商店界面/W_商店菜单.W_商店菜单_C"))
      (bind _output_get_2 (Variables|Default|Set商店菜单 _returnvalue_2))
      (Widget|SetVisibility _output_get_2 "Collapsed")
      (UserInterface|Viewport|AddtoViewport (Variables|Default|Get商店菜单) 0))
    (:then_2
      (bind _returnvalue_3 (UserInterface|CreateWidget "/Game/UMG界面/药品界面/W_背包.W_背包_C"))
      (bind _output_get_3 (Variables|Default|Set背包菜单 _returnvalue_3))
      (Widget|SetVisibility _output_get_3 "Collapsed")
      (UserInterface|Viewport|AddtoViewport (Variables|Default|Get背包菜单) 0))
    (:then_3
      (bind _returnvalue_4 (UserInterface|CreateWidget "/Game/ESC/UI_ECS.UI_ECS_C"))
      (bind _output_get_4 (Variables|Default|SetUI _returnvalue_4))
      (Widget|SetVisibility _output_get_4 "Hidden")
      (UserInterface|Viewport|AddtoViewport (Variables|Default|GetUI) 0))
    (:then_4
      (bind _returnvalue_5 (UserInterface|CreateWidget "/Game/ESC/UI_ECS.UI_ECS_C"))
      (bind _output_get_5 (Variables|Default|Set过关 _returnvalue_5))
      (Widget|SetVisibility _output_get_5 "Hidden")
      (UserInterface|Viewport|AddtoViewport (Variables|Default|Get过关) 0))))

(fn ConstructionScript)