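; BP_子弹_2 is a projectile (bullet) actor with a Paper2D flipbook visual and a fixed initial speed set in the construction script.
; Tick reapplies the 头 flipbook every frame and starts a short delay that ends in destroying the actor.
; Sphere overlap checks for the player's Box component but takes no action.
; BeginPlay caches the player character, and the 子弹速度 and 初始化 functions are empty.
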(event OnComponentBeginOverlap(Sphere)
  (params (OverlappedComponent :type Primitive%20Component%20Object%20Reference) (OtherActor :type Actor%20Object%20Reference) (OtherComp :type Primitive%20Component%20Object%20Reference) (OtherBodyIndex :type Integer) (bFromSweep :type Boolean) (SweepResult :type Hit%20Result%20Structure%20%28by%20ref%29))
  (bind _asbp_player (Utilities|Casting|CastTobp_player OtherActor))
  (if (== (Variables|/Game/blueprints/bp_player.bp_player_C|GetBox _asbp_player) OtherComp)
    _))

(event EventBeginPlay
  (Variables|Default|Set玩家映射 (.AsBp%20Player (Utilities|Casting|CastTobp_player (Game|GetPlayerCharacter 0)))))

(event EventTick
  (params (DeltaSeconds :type Float%20%28single-precision%29))
  (Utilities|FlowControl|Sequence
    (:then_0
      (Sprite|SetFlipbook (Variables|Default|GetPaperFlipbook) "/Game/JDVC/png/enemys/Skeleetons/White/头.头"))
    (:then_1
      (Utilities|FlowControl|Delay 4.0)
      (Actor|DestroyActor))))

(fn ConstructionScript
  (Variables|/Script/Engine.ProjectileMovementComponent|SetInitialSpeed (Variables|Default|GetProjectileMovement) 3e+02))

(fn 子弹速度)

(fn 初始化)