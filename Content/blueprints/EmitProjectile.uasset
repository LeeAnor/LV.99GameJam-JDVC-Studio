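; EmitProjectile is an actor that periodically fires a BP_子弹 bullet while the player character is a bp_player.
; A looping two-second timer spawns the bullet at the actor's location, passing it the player's current weapon state (武器状态).
; Tick turns the Arrow component toward the player pawn, but spawn rotation comes from the actor's rotation with a 90-degree roll offset, not from the Arrow.
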(event Custom|EmitProjectile
  (bind _returnvalue (Transformation|GetActorRotation))
  (bind (_roll _pitch _yaw) (Math|Rotator|BreakRotator _returnvalue))
  (bind _asbp_player (Utilities|Casting|CastTobp_player (Game|GetPlayerCharacter 0)))
  (Development|PrintText "emit")
  (Game|SpawnActorfromClass "/Game/blueprints/BP_子弹.BP_子弹_C" (Math|Transform|MakeTransform (Transformation|GetActorLocation) (Math|Rotator|MakeRotator (- _roll 9e+01) _pitch _yaw)) "Undefined" 0 (Variables|/Game/blueprints/bp_player.bp_player_C|Get武器状态 _asbp_player) 0))

(event EventBeginPlay
  (Utilities|Time|SetTimerbyEvent (delegate Custom|EmitProjectile) 2.0 true))

(event EventTick
  (params (DeltaSeconds :type Float%20%28single-precision%29))
  (bind _returnvalue (Game|Player|GetPlayerPawn 0))
  (Utilities|IsValid _returnvalue
    (:Is%20Valid
      (Transformation|SetWorldRotation (Variables|Default|GetArrow) (Math|Rotator|FindLookatRotation (Transformation|GetActorLocation) (Transformation|GetActorLocation _returnvalue)) false false))))

(fn ConstructionScript)