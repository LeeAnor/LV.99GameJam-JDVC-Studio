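; BP_wuqishangdian is a weapon shop actor with a trigger box and a widget component showing the shop UI.
; On BeginPlay it writes its Name into the 武器商店 widget's title text.
; Box overlap with bp_player toggles widget visibility and the player's in-shop flag (是否在武器商店中).
; On both enter and exit it refreshes each weapon slot in the player's inventory component (BPC库存组件).
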(event OnComponentBeginOverlap(Box)
  (params (OverlappedComponent :type Primitive%20Component%20Object%20Reference) (OtherActor :type Actor%20Object%20Reference) (OtherComp :type Primitive%20Component%20Object%20Reference) (OtherBodyIndex :type Integer) (bFromSweep :type Boolean) (SweepResult :type Hit%20Result%20Structure%20%28by%20ref%29))
  (bind _asbp_player (Utilities|Casting|CastTobp_player OtherActor))
  (Rendering|SetVisibility (Variables|Default|GetWidget) true false)
  (Variables|/Game/blueprints/bp_player.bp_player_C|Set是否在武器商店中 _asbp_player true)
  (for (_ _array_index) (Variables|/Game/UMG界面/BPC_库存组件.BPC_库存组件_C|Get武器名称 (Variables|/Game/blueprints/bp_player.bp_player_C|GetBPC_库存组件 _asbp_player))
    (Default|更新库存格子 (Variables|/Game/blueprints/bp_player.bp_player_C|GetBPC_库存组件 _asbp_player) _array_index)))

(event OnComponentEndOverlap(Box)
  (params (OverlappedComponent :type Primitive%20Component%20Object%20Reference) (OtherActor :type Actor%20Object%20Reference) (OtherComp :type Primitive%20Component%20Object%20Reference) (OtherBodyIndex :type Integer))
  (bind _asbp_player (Utilities|Casting|CastTobp_player OtherActor))
  (Rendering|SetVisibility (Variables|Default|GetWidget) false false)
  (Variables|/Game/blueprints/bp_player.bp_player_C|Set是否在武器商店中 _asbp_player false)
  (for (_ _array_index) (Variables|/Game/UMG界面/BPC_库存组件.BPC_库存组件_C|Get武器名称 (Variables|/Game/blueprints/bp_player.bp_player_C|GetBPC_库存组件 _asbp_player))
    (Default|更新库存格子 (Variables|/Game/blueprints/bp_player.bp_player_C|GetBPC_库存组件 _asbp_player) _array_index)))

(event EventBeginPlay
  (bind _as武器商店 (Utilities|Casting|CastTo武器商店 (UserInterface|GetUserWidgetObject (Variables|Default|GetWidget))))
  (Rendering|Components|TextRender|SetText (Variables|/Game/UMG界面/对话系统/武器商店.武器商店_C|GetNAME _as武器商店) (Variables|Default|Getname)))

(event Collision|EventActorBeginOverlap
  (params (OtherActor :type Actor%20Object%20Reference)))

(event EventTick
  (params (DeltaSeconds :type Float%20%28single-precision%29)))

(fn ConstructionScript)