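; Player character with flipbook animation, Enhanced Input movement and mouse aiming that sets facing and rotates the held weapon.
; Keys 1/2 load weapon data table rows, and Tick sets the matching weapon child actor class from the ID.
; Holding left mouse loops a fire-rate timer that computes a spread transform and calls the weapon's attack, leaving local bullet spawns unwired.
; A breathing toggle gradually raises a pressure value, printed with its state.
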(event Custom|连发
  (bind _returnvalue (Transformation|GetActorLocation))
  (bind _returnvalue_2 (Game|GetPlayerController 0))
  (bind _鼠标位置 (Variables|Default|Get鼠标位置))
  (bind _武器状态 (Variables|Default|Get武器状态))
  (bind _worldlocation (Game|Player|ConvertMouseLocationToWorldSpace _returnvalue_2))
  (bind _returnvalue_3 (Math|Float|MapRangeClamped _鼠标位置 -1.8e+02 -9e+01 1.8e+02 2.7e+02))
  (bind _returnvalue_4 (- _worldlocation _returnvalue))
  (bind _returnvalue_5 (Math|Vector|Normalize (Math|Vector|MakeVector (.x _returnvalue_4) (.y _returnvalue_4) 0.0)))
  (bind _returnvalue_6 (* _returnvalue_5 23.0))
  (bind _returnvalue_7 (+ _returnvalue_6 _returnvalue))
  ;[1 1 1] 连发
  (if (> _鼠标位置 -9e+01)
    (Variables|Default|Set偏移浮点 (Math|Random|RandomFloatinRange (- _鼠标位置 (.子弹偏移 _武器状态)) (+ _鼠标位置 (.子弹偏移 _武器状态))))
    (Variables|Default|Set变换位置 (Math|Transform|MakeTransform _returnvalue_7 (Math|Rotator|MakeRotator 0.0 0.0 (Variables|Default|Get偏移浮点))))
    (else
      (Variables|Default|Set偏移浮点 (Math|Random|RandomFloatinRange (- _returnvalue_3 (.子弹偏移 _武器状态)) (+ _returnvalue_3 (.子弹偏移 _武器状态))))
      (Variables|Default|Set变换位置 (Math|Transform|MakeTransform _returnvalue_7 (Math|Rotator|MakeRotator 0.0 0.0 (Variables|Default|Get偏移浮点))))))
  (Default|WeaponAttack01 (Variables|Default|Get武器)))

(event Custom|停止动画
  ;[1 1 1] idle
  (if (Variables|Default|Get左右速度>0?)
    (Variables|Default|Set玩家动画 "NewEnumerator11")
    (else
      (Variables|Default|Set玩家动画 "NewEnumerator10"))))

(event Custom|更新动画
  (bind _武器状态 (Variables|Default|Get武器状态))
  (bind _scene (Variables|Default|GetScene))
  (Utilities|FlowControl|Sequence
    (:then_0
      ;[1 1 1] 玩家动画
      (switch Utilities|FlowControl|Switch|SwitchonE_行为 (Variables|Default|Get玩家动画)
        (:NewEnumerator8
          (Transformation|SetRelativeRotation (Variables|Default|GetSprite) "0.000000,180.000000,0.000000" false false)
          (Sprite|SetFlipbook (Variables|Default|GetSprite) "/Game/walk/gunwalk/gun_walk.gun_walk"))
        (:NewEnumerator9
          (Transformation|SetRelativeRotation (Variables|Default|GetSprite) "0, 0, 0" false false)
          (Sprite|SetFlipbook (Variables|Default|GetSprite) "/Game/walk/gunwalk/gun_walk.gun_walk"))
        (:NewEnumerator10
          (Transformation|SetRelativeRotation (Variables|Default|GetSprite) "0.000000,180.000000,0.000000" false false)
          (Sprite|SetFlipbook (Variables|Default|GetSprite) "/Game/walk/player1/idle.idle"))
        (:NewEnumerator11
          (Transformation|SetRelativeRotation (Variables|Default|GetSprite) "0, 0, 0" false false)
          (Sprite|SetFlipbook (Variables|Default|GetSprite) "/Game/walk/player1/idle.idle"))))
    (:then_1
      ;[1 1 1] 更改武器角度
      (CallFunction|鼠标位置更改人物方向和武器方向)
      (if true
        (if (Variables|Default|Get左右速度>0?)
          (if true
            (Transformation|SetRelativeRotation (Variables|Default|GetScene) (Math|Rotator|MakeRotator 0.0 (Variables|Default|Get武器位置) 0.0) false false)
            (Transformation|SetRelativeLocation _scene "8.000000,1.000000,-2.000000" false false))
          (else
            (Transformation|SetRelativeRotation _scene (Math|Rotator|MakeRotator 0.0 (Variables|Default|Get武器位置) 0.0) false false)
            (Transformation|SetRelativeLocation _scene "-6.000000,1.000000,-1.000000" false false)))))
    (:then_2
      (if (not (Variables|Default|Get输入检测))
        (CallFunction|停止动画)))
    (:then_3
      (if (Variables|Default|Get压力判断)
        (Utilities|FlowControl|Delay 0.05)
        (CallFunction|增加压力值)))
    (:then_4
      (if (== (.武器id _武器状态) 2.0)
        (Utilities|新建宏 "/Game/blueprints/子弹/BP_武器1.BP_武器1_C")
        (elif (== (.武器id _武器状态) 1.0)
          (Utilities|新建宏 "/Game/blueprints/子弹/BP_武器2.BP_武器2_C"))))))

(event Input|EnhancedActionEvents|EnhancedInputAction移动
  (params (ActionValue :type Vector%202D%20Structure) (ElapsedSeconds :type Float%20%28double-precision%29) (TriggeredSeconds :type Float%20%28double-precision%29) (InputAction :type Input%20Action%20Object%20Reference :default "/Game/input/移动.移动"))
  ;[1 1 1] 移动动画
  (:Triggered
    (Variables|Default|Set输入检测 true)
    (Variables|Default|Set上下 (.x ActionValue))
    (Variables|Default|Set左右 (.y ActionValue))
    (Utilities|FlowControl|Sequence
      (:then_0
        (Pawn|Input|AddMovementInput "0.000000,-1.000000,0.000000" (.x ActionValue) false))
      (:then_1
        (Pawn|Input|AddMovementInput "1.000000,0.000000,0.000000" (.y ActionValue) false)))
    (if (or (!= (.x ActionValue) 0.0) (!= (.y ActionValue) 0.0))
      (if (Variables|Default|Get左右速度>0?)
        (Variables|Default|Set玩家动画 "NewEnumerator9")
        (else
          (Variables|Default|Set玩家动画 "NewEnumerator8")))))
  (:Completed
    (Variables|Default|Set输入检测 false)))

(event Input|EnhancedActionEvents|EnhancedInputAction切换呼吸
  (params (ActionValue :type Boolean) (ElapsedSeconds :type Float%20%28double-precision%29) (TriggeredSeconds :type Float%20%28double-precision%29) (InputAction :type Input%20Action%20Object%20Reference :default "/Game/input/切换呼吸.切换呼吸"))
  (:Triggered
    (Utilities|FlowControl|DoOnce false :!label _label
      (:Completed
        (if (Variables|Default|Get压力判断)
          (Variables|Default|Set压力判断 false)
          (else
            (Variables|Default|Set压力判断 true))))))
  (:Completed
    (goto _label Reset)))

(event EventBeginPlay
  ;[1 1 1] 允许输入
  (CallFunction|开始运行)
  (bind _asbp_playercontrol (Utilities|Casting|CastTobp_playercontrol (Game|GetPlayerController 0)))
  (Variables|Default|Set玩家控制器映射 _asbp_playercontrol)
  (bind _returnvalue (Utilities|GetDataTableRow "/Game/枚举值/武器数据.武器数据" "002")
    (:then
      (Variables|Default|Set武器状态 _returnvalue))))

(event EventTick
  (params (DeltaSeconds :type Float%20%28single-precision%29))
  ;[1 1 1] 每帧
  (CallFunction|获取鼠标位置)
  (CallFunction|更正武器位置)
  (CallFunction|更新动画))

(event Input|MouseEvents|LeftMouseButton
  (params (Key :type Key%20Structure :default "None"))
  (bind _武器状态 (Variables|Default|Get武器状态))
  (:Pressed
    (Utilities|FlowControl|Delay 0.05)
    (bind _returnvalue (Utilities|Time|SetTimerbyEvent (delegate Custom|连发) (.武器射速 _武器状态) true (* (.武器射速 _武器状态) -1.0))))
  (:Released
    (Utilities|Time|ClearandInvalidateTimerbyHandle _returnvalue)))

(event Input|KeyboardEvents|1
  (params (Key :type Key%20Structure :default "None"))
  (:Pressed
    (bind _returnvalue (Utilities|GetDataTableRow "/Game/枚举值/武器数据.武器数据" "001")
      (:then
        (Variables|Default|Set武器状态 _returnvalue)))))

(event Input|KeyboardEvents|2
  (params (Key :type Key%20Structure :default "None"))
  (:Pressed
    (bind _returnvalue (Utilities|GetDataTableRow "/Game/枚举值/武器数据.武器数据" "002")
      (:then
        (Variables|Default|Set武器状态 _returnvalue)))))

(fn ConstructionScript)

(fn 开始运行
  (Utilities|FlowControl|Sequence
    (:then_0
      (bind _asbp_playercontrol (Utilities|Casting|CastTobp_playercontrol (Game|GetPlayerController 0)))
      (Utilities|IsValid (PlayerController|LocalPlayerSubsystems|GetEnhancedInputLocalPlayerSubsystem _asbp_playercontrol)
        (:Is%20Valid
          (Input|AddMappingContext (PlayerController|LocalPlayerSubsystems|GetEnhancedInputLocalPlayerSubsystem _asbp_playercontrol) "/Game/input/综合.综合" 0 "(bIgnoreAllPressedKeysUntilRelease=True,bForceImmediately=False)")
          (Utilities|新建宏 "/Game/blueprints/子弹/BP_武器1.BP_武器1_C"))))))

(fn 获取鼠标位置
  (bind _output_get (Variables|Default|Set鼠标位置 (.yaw (Math|Rotator|FindLookatRotation (Transformation|GetActorLocation) (.WorldLocation (Game|Player|ConvertMouseLocationToWorldSpace (Game|GetPlayerController 0)))))))
  (return _output_get))

(fn 更正武器位置
  (bind _鼠标位置 (Variables|Default|Get鼠标位置))
  (if (< _鼠标位置 0.0)
    (Variables|Default|Set武器位置 (Math|Float|MapRangeClamped _鼠标位置 0.0 -1.8e+02 0.0 1.8e+02))
    (else
      (Variables|Default|Set武器位置 (Math|Float|MapRangeClamped _鼠标位置 0.0 1.8e+02 0.0 -1.8e+02)))))

(fn 人物武器和朝向是否相反
  (if (or (and (Variables|Default|Get左右速度>0?) (Math|Float|InRange(Float) (Variables|Default|Get武器位置) -9e+01 9e+01)) (and (or (Math|Float|InRange(Float) (Variables|Default|Get武器位置) -1.8e+02 -9e+01) (Math|Float|InRange(Float) (Variables|Default|Get武器位置) 9e+01 1.8e+02)) (not (Variables|Default|Get左右速度>0?))))
    _
    (else
      (if (Variables|Default|Get左右速度>0?)
        (if (> (Variables|Default|Get鼠标位置) 0.0)
          (Variables|Default|Set武器位置 -9e+01 :!label _label)
          (else
            (Variables|Default|Set武器位置 9e+01 :!label _label_2)))
        (elif (> (Variables|Default|Get鼠标位置) 0.0)
          (goto _label)
          (else
            (goto _label_2))))
      (Transformation|SetRelativeRotation (Variables|Default|GetScene) (Math|Rotator|MakeRotator 0.0 (Variables|Default|Get武器位置) 0.0) false false)))
  (return (or (and (Variables|Default|Get左右速度>0?) (Math|Float|InRange(Float) (Variables|Default|Get武器位置) -9e+01 9e+01)) (and (or (Math|Float|InRange(Float) (Variables|Default|Get武器位置) -1.8e+02 -9e+01) (Math|Float|InRange(Float) (Variables|Default|Get武器位置) 9e+01 1.8e+02)) (not (Variables|Default|Get左右速度>0?))))))

(fn 鼠标位置更改人物方向和武器方向
  (if (Math|Float|InRange(Float) (Variables|Default|Get武器位置) -9e+01 9e+01)
    (Variables|Default|Set切换武器 "NewEnumerator3")
    (Variables|Default|Set左右速度>0? true)
    (else
      (Variables|Default|Set切换武器 "NewEnumerator2")
      (Variables|Default|Set左右速度>0? false))))

(fn 增加压力值
  (if (<= (Variables|Default|Get压力值) 99.0)
    (Variables|Default|Set压力值 (+ (Variables|Default|Get压力值) 1.0)))
  (if (> (Variables|Default|Get压力值) 5e+01)
    (if (> (Variables|Default|Get压力值) 9e+01)
      (Development|PrintString (Utilities|String|Append "此时极端状态，压力值为：" (Utilities|String|ToString(Float) (Variables|Default|Get压力值))))
      (else
        (Development|PrintString (Utilities|String|Append "此时压力状态，压力值为：" (Utilities|String|ToString(Float) (Variables|Default|Get压力值))))))
    (else
      (Development|PrintString (Utilities|String|Append "此时普通状态，压力值为：" (Utilities|String|ToString(Float) (Variables|Default|Get压力值)))))))

(fn 初始化
  (Variables|/Script/Engine.CharacterMovementComponent|SetMaxWalkSpeed (Variables|Character|GetCharacterMovement) (Variables|/Game/全局变量/BP_GAMEINSTANCE.BP_GAMEINSTANCE_C|Getspeed (.AsBP%20GAMEINSTANCE (Utilities|Casting|CastToBP_GAMEINSTANCE (Game|GetGameInstance))))))