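; BP_子弹 is a bullet projectile actor with a Paper2D flipbook visual, configured by the S武器 weapon struct.
; The construction script sets ProjectileMovement's initial speed from the struct's bullet speed.
; BeginPlay applies the bullet flipbook and destroys the actor after the struct's lifetime.
; The Sphere overlap event and the 子弹速度 function are empty, so the file defines no hit response.
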(event OnComponentBeginOverlap(Sphere)
  (params (OverlappedComponent :type Primitive%20Component%20Object%20Reference) (OtherActor :type Actor%20Object%20Reference) (OtherComp :type Primitive%20Component%20Object%20Reference) (OtherBodyIndex :type Integer) (bFromSweep :type Boolean) (SweepResult :type Hit%20Result%20Structure%20%28by%20ref%29)))

(event EventBeginPlay
  (bind _s_武器 (Variables|Default|Gets_武器))
  (bind (_命名 _弹夹 _子弹速度 _子弹伤害 _子弹偏移 _子弹是否可以穿透 _子弹贴图 _武器射速 _生命时长) (Utilities|Struct|Break武器状态 _s_武器))
  (Utilities|FlowControl|Sequence
    (:then_0
      (Sprite|SetFlipbook (Variables|Default|GetPaperFlipbook) _子弹贴图))
    (:then_1
      (Utilities|FlowControl|Delay _生命时长)
      (Actor|DestroyActor))))

(fn ConstructionScript
  (Variables|/Script/Engine.ProjectileMovementComponent|SetInitialSpeed (Variables|Default|GetProjectileMovement) (.子弹速度 (Variables|Default|Gets_武器))))

(fn 子弹速度)