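; BP_道具1 is a consumable item actor, filed with the medicine UI, that fully heals the player when used.
; Its 使用道具效果 (use item effect) event sets 当前HP (current HP) on bp_player to 最大HP (max HP).
; It then sets the 使用道具成功 (use succeeded) flag to true, with no check on current health.
; The construction script only calls its parent, and the default events are disabled.
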(event EventBeginPlay
  (|CallParentFunction) ; 此节点被禁用，将不会被调用。\n从引脚连出引线来编译功能。
)

(event Collision|EventActorBeginOverlap
  (params (OtherActor :type Actor%20Object%20Reference))
  (|CallParentFunction OtherActor) ; 此节点被禁用，将不会被调用。\n从引脚连出引线来编译功能。
)

(event EventTick
  (params (DeltaSeconds :type Float%20%28single-precision%29))
  (|CallParentFunction DeltaSeconds) ; 此节点被禁用，将不会被调用。\n从引脚连出引线来编译功能。
)

(event Event使用道具效果
  (bind _returnvalue (Game|GetPlayerCharacter 0))
  (bind _asbp_player (Utilities|Casting|CastTobp_player _returnvalue))
  (Variables|/Game/blueprints/bp_player.bp_player_C|Set当前HP _asbp_player (Variables|/Game/blueprints/bp_player.bp_player_C|Get最大HP _asbp_player))
  (Variables|Default|Set使用道具成功 true))

(fn ConstructionScript
  (|CallParentFunction))