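; Potion inventory component that manages the player's potion slots and feeds the shop's potion listing.
; Slot data lives in the GameInstance potion array, resized on BeginPlay, and each change refreshes the matching backpack grid widget.
; Adding fills partial stacks, then empty slots, recursing on overflow using the item class's stack limit.
; Using an item finds or spawns its actor, runs its effect and decrements the slot on success.
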(event EventBeginPlay
  (bind _returnvalue (Game|GetPlayerController 0))
  (bind _asbp_playercontrol (Utilities|Casting|CastTobp_playercontrol _returnvalue))
  (Utilities|Array|Resize (Variables|/Game/全局变量/BP_GAMEINSTANCE.BP_GAMEINSTANCE_C|Get药水数据 (.AsBP%20GAMEINSTANCE (Utilities|Casting|CastToBP_GAMEINSTANCE (Game|GetGameInstance)))) (Variables|/Game/blueprints/bp_playercontrol.bp_playercontrol_C|Get物品格子 _asbp_playercontrol))
  (Variables|Default|Set背包菜单 (Variables|/Game/blueprints/bp_playercontrol.bp_playercontrol_C|Get背包菜单 _asbp_playercontrol))
  (Utilities|FlowControl|Delay 0.2)
  (for (_ _array_index) (Variables|Default|Get药水名称)
    (CallFunction|更新商店格子 _array_index)))

(event EventTick
  (params (DeltaSeconds :type Float%20%28single-precision%29)))

(fn 添加道具
  (params (item :type BP%20道具主类%20Class%20Reference) (数量 :type Integer))
  (bind (_成功 _索引) (CallFunction|查找空格子))
  (bind _returnvalue (Game|GetGameInstance))
  (bind (_成功_2 _索引_2) (CallFunction|查找空格子))
  (bind _asbp_gameinstance (Utilities|Casting|CastToBP_GAMEINSTANCE _returnvalue))
  (bind _药水数据 (Variables|/Game/全局变量/BP_GAMEINSTANCE.BP_GAMEINSTANCE_C|Get药水数据 _asbp_gameinstance))
  (Variables|Default|Set道具 item)
  (Variables|Default|Set数量 数量)
  (Variables|Default|Set叠加数 (.叠加数 (Utilities|Struct|Break药水名称和图标 (.药水 (Utilities|GetClassDefaults (Variables|Default|Get道具))))))
  (if (> (.叠加数 (Utilities|Struct|Break药水名称和图标 (.药水 (Utilities|GetClassDefaults (Variables|Default|Get道具))))) 1)
    (bind _索引_3 (CallFunction|检查空间格子 (Variables|Default|Get道具)))
    (if (Variables|Default|Get是否成功一样)
      (Variables|Default|Set哪个格子 _索引_3)
      (if (> (+ (.amount数量 (CallFunction|获取道具索引 _索引_3)) (Variables|Default|Get数量)) (Variables|Default|Get叠加数))
        (Variables|Default|Set数量 (- (+ (.amount数量 (CallFunction|获取道具索引 _索引_3)) (Variables|Default|Get数量)) (Variables|Default|Get叠加数)))
        (Utilities|Array|SetArrayElem (Variables|/Game/全局变量/BP_GAMEINSTANCE.BP_GAMEINSTANCE_C|Get药水数据 (.AsBP%20GAMEINSTANCE (Utilities|Casting|CastToBP_GAMEINSTANCE (Game|GetGameInstance)))) (Variables|Default|Get哪个格子) (Utilities|Struct|Make药水数据 (Variables|Default|Get道具) (Variables|Default|Get叠加数)))
        (CallFunction|更新库存格子 (Variables|Default|Get哪个格子))
        (bind _余数 (CallFunction|添加道具 (Variables|Default|Get道具) (Variables|Default|Get数量)))
        (return true _余数)
        (else
          (Utilities|Array|SetArrayElem (Variables|/Game/全局变量/BP_GAMEINSTANCE.BP_GAMEINSTANCE_C|Get药水数据 (.AsBP%20GAMEINSTANCE (Utilities|Casting|CastToBP_GAMEINSTANCE (Game|GetGameInstance)))) (Variables|Default|Get哪个格子) (Utilities|Struct|Make药水数据 (Variables|Default|Get道具) (+ (.amount数量 (CallFunction|获取道具索引 _索引_3)) (Variables|Default|Get数量))))
          (CallFunction|更新库存格子 (Variables|Default|Get哪个格子))
          (return true 0)))
      (elif _成功_2
        (Variables|Default|Set哪个格子 _索引_2)
        (if (> (Variables|Default|Get数量) (Variables|Default|Get叠加数))
          ;[1 1 1] 当物品数大于叠加数时
          (Utilities|Array|SetArrayElem _药水数据 (Variables|Default|Get哪个格子) (Utilities|Struct|Make药水数据 (Variables|Default|Get道具) (Variables|Default|Get叠加数)))
          (CallFunction|更新库存格子 (Variables|Default|Get哪个格子))
          (bind _余数_2 (CallFunction|添加道具 (Variables|Default|Get道具) (- (Variables|Default|Get数量) (Variables|Default|Get叠加数))))
          (return true _余数_2)
          (else
            ;[1 1 1] 物品数小于叠加数
            (Utilities|Array|SetArrayElem _药水数据 (Variables|Default|Get哪个格子) (Utilities|Struct|Make药水数据 (Variables|Default|Get道具) (Variables|Default|Get数量)))
            (CallFunction|更新库存格子 (Variables|Default|Get哪个格子))
            (return true 0)))
        (else
          (return false (Variables|Default|Get数量)))))
    (elif _成功
      (bind _output_get (Variables|Default|Set哪个格子 _索引))
      (Utilities|Array|SetArrayElem (Variables|/Game/全局变量/BP_GAMEINSTANCE.BP_GAMEINSTANCE_C|Get药水数据 (.AsBP%20GAMEINSTANCE (Utilities|Casting|CastToBP_GAMEINSTANCE (Game|GetGameInstance)))) _output_get (Utilities|Struct|Make药水数据 (Variables|Default|Get道具) 1))
      (CallFunction|更新库存格子 (Variables|Default|Get哪个格子))
      (if (> (- (Variables|Default|Get数量) 1) 0)
        (bind _余数_3 (CallFunction|添加道具 (Variables|Default|Get道具) (- (Variables|Default|Get数量) 1)))
        (return true _余数_3)
        (else
          (return true 0)))
      (else
        (Development|PrintString "背包已经满了")
        (return false (Variables|Default|Get数量))))))

(fn 查找空格子
  (bind (_array_element _array_index) (Utilities|Array|ForEachLoopwithBreak (Variables|/Game/全局变量/BP_GAMEINSTANCE.BP_GAMEINSTANCE_C|Get药水数据 (.AsBP%20GAMEINSTANCE (Utilities|Casting|CastToBP_GAMEINSTANCE (Game|GetGameInstance)))) :!label _label)
    (:LoopBody
      (if (Utilities|IsValidClass (.item道具 (Utilities|Struct|Break药水数据 _array_element)))
        (Variables|Default|Set成功找到空格子 false)
        (else
          (Variables|Default|Set成功找到空格子 true)
          (Variables|Default|Set哪个格子 _array_index)
          (goto _label Break))))
    (:Completed
      (return (Variables|Default|Get成功找到空格子) (Variables|Default|Get哪个格子)))))

(fn 获取道具索引
  (params (索引 :type Integer))
  (bind _returnvalue (Game|GetGameInstance))
  (bind _asbp_gameinstance (Utilities|Casting|CastToBP_GAMEINSTANCE _returnvalue))
  (bind _药水数据 (Variables|/Game/全局变量/BP_GAMEINSTANCE.BP_GAMEINSTANCE_C|Get药水数据 _asbp_gameinstance))
  (bind _output (Utilities|Array|Get(acopy) _药水数据 索引))
  (bind (_item道具 _数量) (Utilities|Struct|Break药水数据 _output))
  (return _数量 _item道具))

(fn 更新库存格子
  (params (索引 :type Integer))
  (Default|更新数据 (Utilities|Array|Get(acopy) (Variables|/Game/UMG界面/药品界面/W_物品网格.W_物品网格_C|Get物品格子数组_0 (Variables|/Game/UMG界面/药品界面/W_背包.W_背包_C|GetW_物品网格 (Variables|/Game/blueprints/bp_playercontrol.bp_playercontrol_C|Get背包菜单 (.AsBp%20Playercontrol (Utilities|Casting|CastTobp_playercontrol (Game|GetPlayerController 0)))))) 索引)))

(fn 检查空间格子
  (params (item道具 :type BP%20道具主类%20Class%20Reference))
  (bind (_array_element _array_index) (Utilities|Array|ForEachLoopwithBreak (Variables|/Game/全局变量/BP_GAMEINSTANCE.BP_GAMEINSTANCE_C|Get药水数据 (.AsBP%20GAMEINSTANCE (Utilities|Casting|CastToBP_GAMEINSTANCE (Game|GetGameInstance)))) :!label _label)
    (:LoopBody
      (if (and (== (.item道具 (Utilities|Struct|Break药水数据 _array_element)) item道具) (< (.数量 (Utilities|Struct|Break药水数据 _array_element)) (.叠加数 (.药水 (Utilities|GetClassDefaults item道具)))))
        (Variables|Default|Set是否成功一样 true)
        (LocalVariables|Set哪个格子 _array_index)
        (goto _label Break)
        (else
          (Variables|Default|Set是否成功一样 false))))
    (:Completed
      (return (Variables|Default|Get是否成功一样) (LocalVariables|Get哪个格子)))))

(fn 使用道具
  (params (索引 :type Integer))
  (bind _output_get (LocalVariables|Set本地索引 索引))
  (LocalVariables|Set局部数量 (.amount数量 (CallFunction|获取道具索引 _output_get)))
  (if (> (LocalVariables|Get局部数量) 0)
    (bind _returnvalue (Actor|GetActorOfClass (.道具数据 (CallFunction|获取道具索引 _output_get))))
    (Utilities|IsValid _returnvalue
      (:Is%20Valid
        (Default|使用道具效果 _returnvalue)
        (if (Variables|/Game/UMG界面/药品界面/BP_道具主类.BP_道具主类_C|Get使用道具成功 _returnvalue)
          (CallFunction|移除道具 (LocalVariables|Get本地索引) :!label _label)
          (if (<= (LocalVariables|Get局部数量) 0)
            (Default|关闭道具信息 (Variables|Default|Get背包菜单)))))
      (:Is%20Not%20Valid
        (bind _returnvalue_2 (Game|SpawnActorfromClass (.道具数据 (CallFunction|获取道具索引 _output_get)) (Math|Transform|MakeTransform "0, 0, 0" "0, 0, 0" "1.000000,1.000000,1.000000") "Undefined" 0 0))
        (Default|使用道具效果 _returnvalue_2)
        (if (Variables|/Game/UMG界面/药品界面/BP_道具主类.BP_道具主类_C|Get使用道具成功 _returnvalue_2)
          (goto _label))))))

(fn 移除道具
  (params (索引 :type Integer))
  (bind (_amount数量 _道具数据) (CallFunction|获取道具索引 索引))
  (bind _returnvalue (Game|GetGameInstance))
  (bind _asbp_gameinstance (Utilities|Casting|CastToBP_GAMEINSTANCE _returnvalue))
  (bind _药水数据 (Variables|/Game/全局变量/BP_GAMEINSTANCE.BP_GAMEINSTANCE_C|Get药水数据 _asbp_gameinstance))
  (if (> _amount数量 1)
    (Utilities|Array|SetArrayElem _药水数据 索引 (Utilities|Struct|Make药水数据 _道具数据 (- _amount数量 1)))
    (else
      (Utilities|Array|SetArrayElem :TargetArray _药水数据)))
  (CallFunction|更新库存格子 索引))

(fn 更新商店格子
  (params (索引 :type Integer))
  (Default|更新数据 (Utilities|Array|Get(acopy) (Variables|/Game/UMG界面/药品界面/商店界面/W_商店网格.W_商店网格_C|Get商店格子数组 (Variables|/Game/UMG界面/药品界面/商店界面/W_商店菜单.W_商店菜单_C|GetW_商店网格 (Variables|/Game/blueprints/bp_playercontrol.bp_playercontrol_C|Get商店菜单 (.AsBp%20Playercontrol (Utilities|Casting|CastTobp_playercontrol (Game|GetPlayerController 0)))))) 索引)))

(fn 获取商店道具索引
  (params (索引 :type Integer))
  (bind _药水名称 (Variables|Default|Get药水名称))
  (bind _output (Utilities|Array|Get(acopy) _药水名称 索引))
  (bind (_名称 _图标 _可以使用_ _道具描述 _金币 _叠加数) (Utilities|Struct|Break药水名称和图标 _output))
  (return _名称 _图标 _可以使用_ _道具描述 _金币 _叠加数))