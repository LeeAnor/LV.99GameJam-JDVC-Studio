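; BP_道具2 is an item actor in the potion UI folder that gives the player a timed potion state.
; Its 使用道具效果 (use item effect) event sets 药水状态 (potion state) on bp_player and flags 使用道具成功 (use succeeded).
; A 20-second Delay inside the item then switches the potion state back off.
; The state's gameplay effect is not defined here.
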(event EventBeginPlay
  (|CallParentFunction) ; 此节点被禁用，将不会被调用。\n从引脚连出引线来编译功能。
)

(event Collision|EventActorBeginOverlap
  (params (OtherActor :type Actor%20Object%20Reference))
  (|CallParentFunction OtherActor) ; 此节点被禁用，将不会被调用。\n从引脚连出引线来编译功能。
)

(event EventTick
  (params (DeltaSeconds :type Float%20%28single-precision%29))
  (|CallParentFunction DeltaSeconds) ; 此节点被禁用，将不会被调用。\n从引脚连出引线来编译功能。
)

(event Event使用道具效果
  (bind _returnvalue (Game|GetPlayerCharacter 0))
  (bind _asbp_player (Utilities|Casting|CastTobp_player _returnvalue))
  (Variables|/Game/blueprints/bp_player.bp_player_C|Set药水状态 _asbp_player true)
  (Variables|Default|Set使用道具成功 true)
  (Utilities|FlowControl|Delay 2e+01)
  (Variables|/Game/blueprints/bp_player.bp_player_C|Set药水状态 _asbp_player false))

(fn ConstructionScript
  (|CallParentFunction))