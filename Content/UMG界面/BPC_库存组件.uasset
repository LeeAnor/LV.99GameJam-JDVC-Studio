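; BPC_库存组件 is an inventory component that holds weapon entries and drives the inventory grid UI.
; 获取道具索引 returns an entry's name, icon, in-backpack flag, description and number by index.
; After a short BeginPlay delay, it refreshes each entry's grid slot through bp_playercontrol's inventory menu reference.
; 装备武器 and ADD更新数据 are unfinished stubs.
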(event EventBeginPlay
  (Utilities|FlowControl|Delay 0.2)
  (for (_ _array_index) (Variables|Default|Get武器名称)
    (CallFunction|更新库存格子 _array_index)))

(event EventTick
  (params (DeltaSeconds :type Float%20%28single-precision%29)))

(fn 获取道具索引
  (params (索引 :type Integer))
  (bind _武器名称 (Variables|Default|Get武器名称))
  (bind _output (Utilities|Array|Get(acopy) _武器名称 索引))
  (bind (_名称 _图标 _是否在背包 _道具描述 _编号) (Utilities|Struct|Break武器命称和图标 _output))
  (return _名称 _图标 _是否在背包 _道具描述 _编号))

(fn 更新库存格子
  (params (index :type Integer))
  (Default|更新数据 (Utilities|Array|Get(acopy) (Variables|/Game/UMG界面/W_库存网格.W_库存网格_C|Get格子数组 (Variables|/Game/UMG界面/W_菜单.W_菜单_C|GetW_库存网格 (Variables|/Game/blueprints/bp_playercontrol.bp_playercontrol_C|Get库存菜单ref (.AsBp%20Playercontrol (Utilities|Casting|CastTobp_playercontrol (Game|GetPlayerController 0)))))) index)))

(fn ADD更新数据)

(fn 装备武器)