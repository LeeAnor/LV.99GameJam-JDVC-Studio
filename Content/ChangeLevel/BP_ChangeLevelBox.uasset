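; BP_ChangeLevelBox is a trigger actor that opens the level-change UI when the player enters it.
; Overlapping Box with bp_player shows the mouse cursor, prints a debug "Hello" and adds a new UI_ChangeLevel widget to the viewport.
; A second volume, Box1, shows its Widget component while the player is inside and hides it on exit.
; BeginPlay casts that component's widget to 武器商店 (weapon shop) but does nothing further.
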(event OnComponentBeginOverlap(Box)
  (params (OverlappedComponent :type Primitive%20Component%20Object%20Reference) (OtherActor :type Actor%20Object%20Reference) (OtherComp :type Primitive%20Component%20Object%20Reference) (OtherBodyIndex :type Integer) (bFromSweep :type Boolean) (SweepResult :type Hit%20Result%20Structure%20%28by%20ref%29))
  (Utilities|Casting|CastTobp_player OtherActor)
  (Variables|/Script/Engine.PlayerController|SetbShowMouseCursor (Game|GetPlayerController 0) true)
  (Development|PrintString "Hello")
  (bind _returnvalue (UserInterface|CreateWidget "/Game/ChangeLevel/UI_ChangeLevel.UI_ChangeLevel_C"))
  (UserInterface|Viewport|AddtoViewport _returnvalue 0))

(event OnComponentBeginOverlap(Box1)
  (params (OverlappedComponent :type Primitive%20Component%20Object%20Reference) (OtherActor :type Actor%20Object%20Reference) (OtherComp :type Primitive%20Component%20Object%20Reference) (OtherBodyIndex :type Integer) (bFromSweep :type Boolean) (SweepResult :type Hit%20Result%20Structure%20%28by%20ref%29))
  (Utilities|Casting|CastTobp_player OtherActor)
  (Rendering|SetVisibility (Variables|Default|GetWidget) true false))

(event OnComponentEndOverlap(Box1)
  (params (OverlappedComponent :type Primitive%20Component%20Object%20Reference) (OtherActor :type Actor%20Object%20Reference) (OtherComp :type Primitive%20Component%20Object%20Reference) (OtherBodyIndex :type Integer))
  (Utilities|Casting|CastTobp_player OtherActor)
  (Rendering|SetVisibility (Variables|Default|GetWidget) false false))

(event EventBeginPlay
  (Utilities|Casting|CastTo武器商店 (UserInterface|GetUserWidgetObject (Variables|Default|GetWidget))))

(event Collision|EventActorBeginOverlap
  (params (OtherActor :type Actor%20Object%20Reference)))

(event EventTick
  (params (DeltaSeconds :type Float%20%28single-precision%29)))

(fn ConstructionScript)